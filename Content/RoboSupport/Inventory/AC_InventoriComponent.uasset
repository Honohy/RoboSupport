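; AC_InventoriComponent is an inventory component that keeps an array of item structures and stacks added items.
; AddItem calls FindeItem to match by Type, then overwrites that slot with a summed Amount or appends a new entry.
; The sum reads the existing Amount at the incoming item's Index field, while the write uses the found array index.
; Tick prints every item's name and amount as a debug readout.
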(event `self.ReceiveTick`
  (params (DeltaSeconds :type "Float (single-precision)"))
  (for _array_element (`self.Inventory`)
    (bind (_name _amount) (break `/Game/RoboSupport/Inventory/BPS_ItemStructure` _array_element))
    (`KismetSystemLibrary.PrintString` (`KismetStringLibrary.Concat_StrStr` "Item: " (`KismetTextLibrary.Conv_TextToString` _name) " " (`KismetStringLibrary.Conv_IntToString` _amount)) true true (struct :`G` 0.66 :`B` 1.0 :`A` 1.0) 0.0)))

(fn `AddItem`
  (params (ToAdd :type "/Game/RoboSupport/Inventory/BPS_ItemStructure Structure"))
  (bind (_name _amount _index _type _itemclass) (break `/Game/RoboSupport/Inventory/BPS_ItemStructure` ToAdd))
  (bind (_success _item_structure _array_index) (`self.FindeItem` ToAdd))
  (if _success
    (`KismetArrayLibrary.Array_Set` (`self.Inventory`) _array_index (make `/Game/RoboSupport/Inventory/BPS_ItemStructure` _name (+ (`.Amount_6_2053B62740303ECD6EA195ACE482CAD5` (break `/Game/RoboSupport/Inventory/BPS_ItemStructure` (`|GetArrayItem` (`self.Inventory`) _index))) _amount) _index _type _itemclass) true)
    (else
      (`KismetArrayLibrary.Array_Set` (`self.Inventory`) (`KismetArrayLibrary.Array_Length` (`self.Inventory`)) ToAdd true)
      (`KismetSystemLibrary.PrintString` (`KismetStringLibrary.Concat_StrStr` (`KismetTextLibrary.Conv_TextToString` (`.Name_4_47732CD64FE5B42E07CD3B89426A9B06` (break `/Game/RoboSupport/Inventory/BPS_ItemStructure` ToAdd))))))))

(fn `FindeItem`
  (params (ItemToFind :type "/Game/RoboSupport/Inventory/BPS_ItemStructure Structure"))
  (returns (Success :type Boolean) (`Item Structure` :type "/Game/RoboSupport/Inventory/BPS_ItemStructure Structure") (`Array Index` :type Integer))
  (for (_array_element _array_index) (`self.Inventory`)
    (if (`|EnumEquality` (`.Type_11_0BE483C64340C4F290A689A17110FEA8` (break `/Game/RoboSupport/Inventory/BPS_ItemStructure` _array_element)) ItemToFind_Type_11_0BE483C64340C4F290A689A17110FEA8)
      (`KismetSystemLibrary.PrintString` "find")
      (return true (struct) _array_index)))
  (return false (struct) 0))