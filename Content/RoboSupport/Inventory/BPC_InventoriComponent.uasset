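; Inventory component that stores item structures in an array, using each item's own Index as its slot.
; AddItem calls FindeItem, then either adds the amount to the occupied slot or writes the new item and prints its name, growing the array as needed.
; FindeItem treats a slot with an item class set as occupied, without comparing items, and returns that class's defaults.
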(fn `AddItem`
  (params (ToAdd :type "/Game/RoboSupport/Inventory/BPS_ItemStructure Structure"))
  (bind (_name _amount _index) (break `/Game/RoboSupport/Inventory/BPS_ItemStructure` ToAdd))
  (bind (_name_2 _amount_2 _index_2 _type _itemclass) (break `/Game/RoboSupport/Inventory/BPS_ItemStructure` ToAdd))
  (bind _success (`self.FindeItem` ToAdd))
  (if _success
    (`KismetArrayLibrary.Array_Set` (`self.Inventory`) _index_2 (make `/Game/RoboSupport/Inventory/BPS_ItemStructure` _name_2 (+ (`.Amount_6_2053B62740303ECD6EA195ACE482CAD5` (break `/Game/RoboSupport/Inventory/BPS_ItemStructure` (`|GetArrayItem` (`self.Inventory`) _index_2))) _amount_2) _index_2 _type _itemclass) true)
    (else
      (`KismetArrayLibrary.Array_Set` (`self.Inventory`) _index ToAdd true)
      (`KismetSystemLibrary.PrintString` (`KismetStringLibrary.Concat_StrStr` (`KismetTextLibrary.Conv_TextToString` _name))))))

(fn `FindeItem`
  (params (ItemToFind :type "/Game/RoboSupport/Inventory/BPS_ItemStructure Structure"))
  (returns (Success :type Boolean) (`Item Structure` :type "/Game/RoboSupport/Inventory/BPS_ItemStructure Structure"))
  (bind (_output_name _output_amount _output_index _output_type _output_itemclass) (break `/Game/RoboSupport/Inventory/BPS_ItemStructure` (`|GetArrayItem` (`self.Inventory`) ItemToFind_Index_8_4B907A7747A7BA08AB0D5E9B9D173234)))
  (if (!= _output_itemclass null)
    (`KismetSystemLibrary.PrintString` "find")
    (return true (defaults `Object` _output_itemclass))
    (else
      (return false))))