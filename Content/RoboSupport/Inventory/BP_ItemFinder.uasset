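; BP_ItemFinder is an interactable actor that checks whether the player's robot carries a given item, apparently as an inventory test.
; On Interact it casts the player pawn to BP_RobotSupport and queries its inventory component for the FindedItem type with a hardcoded index.
; The result is only printed to screen as a found or not-found message.
; AddCart is a stub that always returns false.
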(event `/Game/RoboSupport/Interface/BPI_Interact.Interact`
  (params (Interactor :type "Actor Object Reference"))
  (bind _asbp_robot_support (cast `/Game/RoboSupport/Characters/BP_RobotSupport` (`GameplayStatics.GetPlayerPawn` 0)))
  (bind _success (`/Game/RoboSupport/Inventory/BPC_InventoriComponent.FindeItem` (`/Game/RoboSupport/Characters/BP_RobotSupport.BPC_InventoriComponent` _asbp_robot_support) (make `/Game/RoboSupport/Inventory/BPS_ItemStructure` "" 0 2 (`self.Finded item`))))
  (if _success
    (`KismetSystemLibrary.PrintString` "have ")
    (else
      (`KismetSystemLibrary.PrintString` "havnt "))))

(fn `AddCart`
  (params (Interactor :type "Actor Object Reference"))
  (returns (NewParam :type Boolean))
  (return false))

(fn `UserConstructionScript`)