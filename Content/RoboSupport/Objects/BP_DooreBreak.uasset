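; BP_DooreBreak is an interactable door that breaks through on the third interaction.
; The first two interactions only play a knock sound and advance a counter.
; The third briefly simulates physics, launching the lightened door with an impulse, then restores a heavy mass, plays a collapse sound and freezes it.
; Later interactions re-enable physics on the heavy door, while the other interaction functions are stubs.
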(event `/Game/RoboSupport/Interface/BPI_Interact.Interact`
  (params (Interactor :type "Actor Object Reference") (CurrentTool :type "/Game/RoboSupport/Inventory/E_Tools Enum" :default "NewEnumerator4") (PbutoonAct :type "/Game/RoboSupport/Puzzle/E_ElemPButtonAct Enum" :default "NewEnumerator0"))
  (bind _door (`self.Door`))
  (bind _door_2 (`self.Door`))
  (bind _door_3 (`self.Door`))
  (if (`self.IsBreakthrough`)
    (if (`self.IsBreakthrough`) :!label _label
      (`PrimitiveComponent.SetSimulatePhysics` _door_3 true)
      (`PrimitiveComponent.SetMassOverrideInKg` _door_3 "None" 500.0 true)
      (else
        (`PrimitiveComponent.SetSimulatePhysics` _door_2 true)
        (`PrimitiveComponent.SetMassOverrideInKg` _door_2 "None" 1.0 true)
        (`PrimitiveComponent.AddImpulse` _door (-1070.0 0.0 0.0) "None" false)
        (`KismetSystemLibrary.Delay` 0.2)
        (`PrimitiveComponent.SetMassOverrideInKg` _door "None" 500.0 true)
        (`GameplayStatics.SpawnSoundAtLocation` "/Game/Downloads/StarterContent/Audio/Collapse_Cue.Collapse_Cue" (`SceneComponent.K2_GetComponentLocation` (`self.Door`)) (struct) 1.0 1.0 0.0 null null)
        (`KismetSystemLibrary.Delay` 0.2)
        (`PrimitiveComponent.SetSimulatePhysics` (`self.Door`) false)
        (set `self.IsBreakthrough` true)))
    (else
      (set `self.KnockCounter` (+ (`self.KnockCounter`) 1))
      (if (== (`self.KnockCounter`) 3)
        (goto _label)
        (else
          (`GameplayStatics.SpawnSoundAtLocation` "/Game/RoboSupport/Objects/Audio/ClosetDoor_Cue.ClosetDoor_Cue" (`SceneComponent.K2_GetComponentLocation` (`self.Door`)) (struct) 1.0 1.0 0.0 null null))))))

(fn `AddCart`
  (params (Interactor :type "Actor Object Reference"))
  (returns (NewParam :type Boolean))
  (return false))

(fn `GetInteractableActions`
  (returns (Actions :type "Map of /Game/RoboSupport/Inventory/E_Tools Enum to String") (PuzzleRef :type "Actor Object Reference"))
  (return _ null))

(fn `GetInteractableType`
  (returns (NewParam :type "/Game/RoboSupport/Objects/E_InteractType Enum"))
  (return "NewEnumerator0"))

(fn `PuzzleInteract`
  (params (AnyTextIn :type String))
  (returns (AnyTextOut :type String))
  (return ""))

(fn `UserConstructionScript`)