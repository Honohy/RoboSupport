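; BP_CodeDoore is an interactable door that opens only for an interactor carrying the required card.
; Interact searches the interactor's inventory component for the CardCheck item; on success, a FlipFlop plays or reverses a timeline that yaws the door.
; Without the card, it shows a configurable warning text widget for three seconds.
; BeginPlay applies a color material to the card indicator, while the other interaction functions are stubs returning defaults.
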(event `/Game/RoboSupport/Interface/BPI_Interact.Interact`
  (params (Interactor :type "Actor Object Reference") (CurrentTool :type "/Game/RoboSupport/Inventory/E_Tools Enum" :default "NewEnumerator4") (PbutoonAct :type "/Game/RoboSupport/Puzzle/E_ElemPButtonAct Enum" :default "NewEnumerator0"))
  (set `self.Interactor` Interactor)
  (bind _success (`/Game/RoboSupport/Inventory/AC_InventoriComponent.FindeItem` (`self.K2_GetComponentsByClass` Interactor "/Game/RoboSupport/Inventory/AC_InventoriComponent.AC_InventoriComponent_C") (make `/Game/RoboSupport/Inventory/BPS_ItemStructure` "" 0 0 (`self.CardCheck`))))
  (if _success
    (`/Engine/EditorBlueprintResources/StandardMacros.FlipFlop`
      (:`A`
        (bind (_direction _doorrotator) (`Timeline|OpenDoore` :!label _label)
          (:`Update`
            (`SceneComponent.K2_SetRelativeRotation` (`self.Door`) (`KismetMathLibrary.MakeRotator` 0.0 0.0 _doorrotator) false false))))
      (:`B`
        (goto _label :!via `Reverse`)))
    (else
      (bind _returnvalue (`|CreateWidget` "/Game/RoboSupport/Objects/Widget/WBP_WarningText.WBP_WarningText_C" (`GameplayStatics.GetPlayerController` 0) (`self.Set Text`) (`self.Specified Color`)))
      (bind _output_get (set `self.ActiveWidget` _returnvalue))
      (`UserWidget.AddToViewport` _output_get 0)
      (`KismetSystemLibrary.Delay` 3.0)
      (`Widget.RemoveFromParent` (`self.ActiveWidget`)))))

(event `self.ReceiveBeginPlay`
  (`PrimitiveComponent.SetMaterial` (`self.CardIndicator`) 0 (`self.IdicatorColor`)))

(fn `AddCart`
  (params (Interactor :type "Actor Object Reference"))
  (returns (NewParam :type Boolean))
  (return false))

(fn `GetInteractableActions`
  (returns (Actions :type "Map of /Game/RoboSupport/Inventory/E_Tools Enum to String") (PuzzleRef :type "Actor Object Reference"))
  (return _ null))

(fn `GetInteractableType`
  (returns (NewParam :type "/Game/RoboSupport/Objects/E_InteractType Enum"))
  (return "NewEnumerator0"))

(fn `PuzzleInteract`
  (params (AnyTextIn :type String))
  (returns (AnyTextOut :type String))
  (return ""))

(fn `UserConstructionScript`)