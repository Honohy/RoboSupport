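; BP_2Card is a card pickup object that the player can collect into their inventory.
; On Interact, it casts the player pawn to BP_RobotSupport and passes its ItemStructure to that pawn's inventory component through AddItem.
; It then destroys itself and prints a debug "added" message, without checking whether the add succeeded.
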(event `/Game/RoboSupport/Interface/BPI_Interact.Interact`
  (params (Interactor :type "Actor Object Reference"))
  (bind _asbp_robot_support (cast `/Game/RoboSupport/Characters/BP_RobotSupport` (`GameplayStatics.GetPlayerPawn` 0)))
  (`/Game/RoboSupport/Inventory/AC_InventoriComponent.AddItem` (`/Game/RoboSupport/Characters/BP_RobotSupport.BPC_InventoriComponent` _asbp_robot_support) (`self.ItemStructure`))
  (`self.K2_DestroyActor`)
  (`KismetSystemLibrary.PrintString` "added"))

(fn `UserConstructionScript`
  (`parent.UserConstructionScript`))