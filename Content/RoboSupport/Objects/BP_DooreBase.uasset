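; Base door actor that players interact with, opening and closing only for interactors carrying a key card.
; Interact searches the interactor's inventory component for a CardCheck item.
; On success, a FlipFlop alternately plays and reverses the OpenDoore timeline, which drives the door's relative yaw.
; The other interaction functions, AddCart, GetInteractableActions and PuzzleInteract, are stubs, while GetInteractableType returns a fixed enum value.
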(event `/Game/RoboSupport/Interface/BPI_Interact.Interact`
  (params (Interactor :type "Actor Object Reference") (CurrentTool :type "/Game/RoboSupport/Inventory/E_Tools Enum" :default "NewEnumerator1") (PbutoonAct :type "/Game/RoboSupport/Puzzle/E_ElemPButtonAct Enum" :default "NewEnumerator0"))
  (bind _success (`/Game/RoboSupport/Inventory/AC_InventoriComponent.FindeItem` (`self.K2_GetComponentsByClass` Interactor "/Game/RoboSupport/Inventory/AC_InventoriComponent.AC_InventoriComponent_C") (make `/Game/RoboSupport/Inventory/BPS_ItemStructure` "" 0 0 (`self.CardCheck`))))
  (if _success
    (`/Engine/EditorBlueprintResources/StandardMacros.FlipFlop`
      (:`A`
        (bind (_direction _doorrotator) (`Timeline|OpenDoore` :!label _label)
          (:`Update`
            (`SceneComponent.K2_SetRelativeRotation` (`self.Door`) (`KismetMathLibrary.MakeRotator` 0.0 0.0 _doorrotator) false false))))
      (:`B`
        (goto _label :!via `Reverse`)))))

(fn `AddCart`
  (params (Interactor :type "Actor Object Reference"))
  (returns (NewParam :type Boolean))
  (return false))

(fn `GetInteractableActions`
  (returns (Actions :type "Map of /Game/RoboSupport/Inventory/E_Tools Enum to String") (PuzzleRef :type "Actor Object Reference"))
  (return _ null))

(fn `GetInteractableType`
  (returns (NewParam :type "/Game/RoboSupport/Objects/E_InteractType Enum"))
  (return "NewEnumerator0"))

(fn `PuzzleInteract`
  (params (AnyTextIn :type String))
  (returns (AnyTextOut :type String))
  (return ""))

(fn `UserConstructionScript`)