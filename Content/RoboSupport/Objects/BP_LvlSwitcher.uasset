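; BP_LvlSwitcher is an interactable level-switch object that opens the level set in LevelToOpen when its Interact event fires.
; The Construction Script writes LevelText to a TextRender component, so the label updates at edit time.
; The other interaction functions (AddCart, GetInteractableActions, GetInteractableType, PuzzleInteract) only return empty or fixed values.
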(event `self.ReceiveBeginPlay`)

(event `/Game/RoboSupport/Interface/BPI_Interact.Interact`
  (params (Interactor :type "Actor Object Reference") (CurrentTool :type "/Game/RoboSupport/Inventory/E_Tools Enum" :default "NewEnumerator4") (PbutoonAct :type "/Game/RoboSupport/Puzzle/E_ElemPButtonAct Enum" :default "NewEnumerator0"))
  (`GameplayStatics.OpenLevelBySoftObjectPtr` (`self.LevelToOpen`)))

(fn `AddCart`
  (params (Interactor :type "Actor Object Reference"))
  (returns (NewParam :type Boolean))
  (return false))

(fn `GetInteractableActions`
  (returns (Actions :type "Map of /Game/RoboSupport/Inventory/E_Tools Enum to String") (PuzzleRef :type "Actor Object Reference"))
  (return _ null))

(fn `GetInteractableType`
  (returns (NewParam :type "/Game/RoboSupport/Objects/E_InteractType Enum"))
  (return "NewEnumerator0"))

(fn `PuzzleInteract`
  (params (AnyTextIn :type String))
  (returns (AnyTextOut :type String))
  (return ""))

(fn `UserConstructionScript`
  (`TextRenderComponent.K2_SetText` (`self.TextRender`) (`self.LevelText`)))