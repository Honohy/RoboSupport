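; Base Blueprint for physical objects, built on a static mesh with a configurable mesh asset and mass.
; The construction script applies the chosen mesh, and BeginPlay overrides the mesh's mass in kilograms.
; It exposes interaction functions that report a fixed interactable type, while the cart, action list and puzzle functions are stubs returning empty or false values.
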(event `self.ReceiveBeginPlay`
  (`PrimitiveComponent.SetMassOverrideInKg` (`self.StaticMesh`) "None" (`self.Mass in Kg`) true))

(fn `AddCart`
  (params (Interactor :type "Actor Object Reference"))
  (returns (NewParam :type Boolean))
  (return false))

(fn `GetInteractableActions`
  (returns (Actions :type "Map of /Game/RoboSupport/Inventory/E_Tools Enum to String") (PuzzleRef :type "Actor Object Reference"))
  (return _ null))

(fn `GetInteractableType`
  (returns (NewParam :type "/Game/RoboSupport/Objects/E_InteractType Enum"))
  (return "NewEnumerator3"))

(fn `PuzzleInteract`
  (params (AnyTextIn :type String))
  (returns (AnyTextOut :type String))
  (return ""))

(fn `UserConstructionScript`
  (`StaticMeshComponent.SetStaticMesh` (`self.StaticMesh`) (`self.SetStaticMesh`)))