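; BP_RobotSupport is a player-controlled robot that drives, looks around, interacts with objects and carries an inventory component.
; Movement is tank-style: forward input offsets the actor, sideways input yaws it, while look input yaws the Head and pitches the Camera.
; Interact runs a short debug-drawn sphere trace from the camera and sends an Interact interface message to the hit actor.
; K and L print inventory checks; AddCart and its own Interact are stubs.
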(event `InputAxis|MoveForward`
  (params (AxisValue :type "Float (single-precision)"))
  ;[1 1 1] Move Forward/Backward
  (`self.K2_AddActorLocalOffset` (`KismetMathLibrary.MakeVector` (* AxisValue (`self.ForwardSpeed`)))))

(event `InputAxis|MoveRight`
  (params (AxisValue :type "Float (single-precision)"))
  ;[1 1 1] Move Right/Left
  (`self.K2_AddActorLocalRotation` (`KismetMathLibrary.MakeRotator` 0.0 0.0 (* AxisValue (`self.TurnSpeed`)))))

(event `InputAxis|Turn`
  (params (AxisValue :type "Float (single-precision)"))
  ;[1 1 1] Rotate view
  (`SceneComponent.K2_AddLocalRotation` (`self.Head`) (`KismetMathLibrary.MakeRotator` 0.0 0.0 AxisValue) false false))

(event `InputAxis|Up`
  (params (AxisValue :type "Float (single-precision)"))
  ;[1 1 1] Rise/lower view
  (`SceneComponent.K2_AddLocalRotation` (`self.Camera`) (`KismetMathLibrary.MakeRotator` 0.0 AxisValue) false false))

(event `Key|K`
  (params (Key :type "Key Structure"))
  (:`Pressed`
    (bind _success (`/Game/RoboSupport/Inventory/BPC_InventoriComponent.FindeItem` (`self.BPC_InventoriComponent`) (make `/Game/RoboSupport/Inventory/BPS_ItemStructure` "")))
    (if _success
      (`KismetSystemLibrary.PrintString` "Foundet Parts"))))

(event `InputAction|Interact`
  (params (Key :type "Key Structure"))
  ;[1 1 1] Interaction
  (:`Pressed`
    (`self.InteractionSystem`)))

(event `Key|L`
  (params (Key :type "Key Structure"))
  (:`Pressed`
    (for _array_element (`/Game/RoboSupport/Inventory/BPC_InventoriComponent.Inventory` (`self.BPC_InventoriComponent`))
      (bind (_name _amount _index _type _itemclass) (break `/Game/RoboSupport/Inventory/BPS_ItemStructure` _array_element))
      (if (!= _itemclass null)
        (`KismetSystemLibrary.PrintString` (`KismetStringLibrary.Concat_StrStr` (`KismetTextLibrary.Conv_TextToString` _name) (`KismetStringLibrary.Conv_IntToString` _amount)))))))

(fn `AddCart`
  (params (Interactor :type "Actor Object Reference"))
  (returns (NewParam :type Boolean))
  (return false))

(fn `Interact`
  (params (Interactor :type "Actor Object Reference"))
  (return))

(fn `InteractionSystem`
  (bind _camera (`self.Camera`))
  (bind _returnvalue (`SceneComponent.K2_GetComponentLocation` _camera))
  (bind (_outhit _returnvalue_2) (`KismetSystemLibrary.SphereTraceSingle` :`Start` _returnvalue :`End` (+ (* (`SceneComponent.GetForwardVector` _camera) 250.0) _returnvalue) :`Radius` 10.0 :`TraceChannel` "TraceTypeQuery1" :`DrawDebugType` "ForDuration"))
  (if _returnvalue_2
    (bind _output_get (set `self.HitResult` _outhit))
    (message `/Game/RoboSupport/Interface/BPI_Interact.Interact` (`.HitActor` (`GameplayStatics.BreakHitResult` _output_get)) null)))

(fn `UserConstructionScript`)