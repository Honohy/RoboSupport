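; Main character Blueprint for RoboSupport that handles player movement with tank-style controls.
; MoveForward offsets the actor along its local X axis by ForwardSpeed, and MoveRight yaws it by TurnSpeed instead of strafing.
; Both apply per axis event without delta-time scaling, so movement depends on frame rate.
; The Turn and Up view inputs do nothing, as their local pitch and yaw rotation nodes are disconnected.
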(event `InputAxis|MoveForward`
  (params (AxisValue :type "Float (single-precision)"))
  ;[1 1 1] Move Forward/Backward
  (`self.K2_AddActorLocalOffset` (`KismetMathLibrary.MakeVector` (* AxisValue (`self.ForwardSpeed`)))))

(event `InputAxis|MoveRight`
  (params (AxisValue :type "Float (single-precision)"))
  ;[1 1 1] Move Right/Left
  (`self.K2_AddActorLocalRotation` (`KismetMathLibrary.MakeRotator` 0.0 0.0 (* AxisValue (`self.TurnSpeed`)))))

(event `InputAxis|Turn`
  (params (AxisValue :type "Float (single-precision)"))
  ;[1 1 1] Rotate view
)

(event `InputAxis|Up`
  (params (AxisValue :type "Float (single-precision)"))
  ;[1 1 1] Rise/lower view
)

(fn `UserConstructionScript`)