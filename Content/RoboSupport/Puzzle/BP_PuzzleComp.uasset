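; BP_PuzzleComp is a puzzle object, apparently a computer, with clickable power supply, power button and motherboard parts.
; Clicking a part passes its action list to the UI call, with a helper that toggles a WBP_test widget at the mouse cursor.
; Tool interactions and power on/off actions charge or discharge the BP_RobotSupport pawn's battery.
; A Problems array holds defect statuses, updated by FixProblem and debug-printed every tick.
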(event `self.ReceiveTick`
  (params (DeltaSeconds :type "Float (single-precision)"))
  (for _array_element (`self.Problems`)
    (bind (_name _status) (break `/Game/RoboSupport/Puzzle/F_defects` _array_element))
    (`KismetSystemLibrary.PrintString` (`KismetStringLibrary.Concat_StrStr` "Name: " _name " Status: " (`KismetStringLibrary.Conv_BoolToString` _status)) true true (struct :`G` 0.66 :`B` 1.0 :`A` 1.0) 0.0)))

(event `self.FixProblem`
  (params (Index :type Integer) (Status :type Boolean))
  (bind _problems (`self.Problems`))
  (`KismetArrayLibrary.Array_Set` _problems Index (make `/Game/RoboSupport/Puzzle/F_defects` (`.Name_10_7756C5F44B5E7448E29089A55EF04FFC` (break `/Game/RoboSupport/Puzzle/F_defects` (`|GetArrayItem` _problems Index))) Status)))

(event `self.SupplyUnit.OnClicked`
  (params (TouchedComponent :type "PrimitiveComponent Object Reference") (ButtonPressed :type "Key Structure"))
  ;[1 1 1] Вызов UI при нажатии на элемент и заполнение UI из массива ENUM
  (`self.CallUIOnClickElem` (`self.ActionSupplyUnit`)))

(event `self.PowerButton.OnClicked`
  (params (TouchedComponent :type "PrimitiveComponent Object Reference") (ButtonPressed :type "Key Structure"))
  ;[1 1 1] Вызов UI при нажатии на элемент и заполнение UI из массива ENUM
  (`self.CallUIOnClickElem` (`self.ActionPowerButton`)))

(event `self.MotherBoard.OnClicked`
  (params (TouchedComponent :type "PrimitiveComponent Object Reference") (ButtonPressed :type "Key Structure"))
  ;[1 1 1] Вызов UI при нажатии на элемент и заполнение UI из массива ENUM
  (`self.CallUIOnClickElem` (`self.ActionMoterboard`)))

(event `self.ReceiveBeginPlay`
  (`PrimitiveComponent.SetRenderCustomDepth` (`self.SupplyUnit`) false)
  (`KismetArrayLibrary.Array_Clear` (`self.ActonPowerButton`))
  (for _array_element (`self.ActionPowerButton`)
    (`KismetArrayLibrary.Array_Add` (`self.ActonPowerButton`) (`|GetEnumeratorNameAsString` _array_element))))

(event `Testword`
  (`KismetSystemLibrary.PrintString` "click" true true (struct :`R` 1.0 :`A` 1.0)))

(event `/Game/RoboSupport/Interface/BPI_Interact.Interact`
  (params (Interactor :type "Actor Object Reference") (CurrentTool :type "/Game/RoboSupport/Inventory/E_Tools Enum" :default "NewEnumerator1") (PbutoonAct :type "/Game/RoboSupport/Puzzle/E_ElemPButtonAct Enum" :default "NewEnumerator0"))
  (bind _returnvalue (`GameplayStatics.GetPlayerPawn` 0))
  (switch `/Game/RoboSupport/Inventory/E_Tools` CurrentTool
    (:`NewEnumerator1`
      (bind _asbp_robot_support (cast `/Game/RoboSupport/Characters/BP_RobotSupport` _returnvalue))
      (`/Game/RoboSupport/Characters/BP_RobotSupport.Battery Disсharge` _asbp_robot_support 10.0))
    (:`NewEnumerator2`
      (bind _asbp_robot_support_2 (cast `/Game/RoboSupport/Characters/BP_RobotSupport` _returnvalue))
      (`/Game/RoboSupport/Characters/BP_RobotSupport.Battery Charge` _asbp_robot_support_2 10.0))))

(event `OnClicked_Event_0`
  ;[1 1 1] Попытка вызвать клик по кнопке интерфейса
)

(event `/Game/RoboSupport/Interface/BPI_Interact.PuzzleElemInteract`
  (params (Interactor :type "Actor Object Reference") (PbutoonAct :type "/Game/RoboSupport/Puzzle/E_ElemPButtonAct Enum" :default "NewEnumerator0"))
  (bind _returnvalue (`GameplayStatics.GetPlayerPawn` 0))
  (switch `/Game/RoboSupport/Puzzle/E_ElemPButtonAct` PbutoonAct
    (:`NewEnumerator0`
      (bind _asbp_robot_support (cast `/Game/RoboSupport/Characters/BP_RobotSupport` _returnvalue))
      (`/Game/RoboSupport/Characters/BP_RobotSupport.Battery Disсharge` _asbp_robot_support 5.0))
    (:`NewEnumerator1`
      (bind _asbp_robot_support_2 (cast `/Game/RoboSupport/Characters/BP_RobotSupport` _returnvalue))
      (`/Game/RoboSupport/Characters/BP_RobotSupport.Battery Charge` _asbp_robot_support_2 5.0))))

(fn `NewFunction_0_0`
  (params (Array :type "Array of /Game/RoboSupport/Puzzle/E_ElemPButtonAct Enum (by ref)"))
  (bind (_locationx _locationy) (`PlayerController.GetMousePosition` (`GameplayStatics.GetPlayerController` 0)))
  (bind _testui (`self.TestUI`)
    (:`then`
      (`Widget.RemoveFromParent` _testui)
      (set `self.TestUI` null))
    (:`else`
      (bind _returnvalue (`|CreateWidget` "/Game/RoboSupport/Puzzle/Widget/WBP_test.WBP_test_C" null self))
      (bind _output_get (set `self.TestUI` _returnvalue))
      (`UserWidget.AddToViewport` _output_get 0)
      (`/Game/RoboSupport/Puzzle/Widget/WBP_test.FillData` (`self.TestUI`) Array)
      ;[1 1 1] Вызов виджета рядом с курсором мышки
      (`UserWidget.SetPositionInViewport` (`self.TestUI`) (`KismetMathLibrary.MakeVector2D` _locationx _locationy) true))))

(fn `UserConstructionScript`
  (`parent.UserConstructionScript`))