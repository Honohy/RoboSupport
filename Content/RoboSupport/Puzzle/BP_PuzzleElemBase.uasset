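; BP_PuzzleElemBase is a base Blueprint for puzzle elements that highlights on cursor hover.
; Begin and end cursor-over events on the Body component toggle its Render Custom Depth flag.
; GetInteractableType, GetInteractableActions, PuzzleInteract and AddCart are stubs returning default values: first enum entry, no actions, empty text and false.
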(event `self.Body.OnBeginCursorOver`
  (params (TouchedComponent :type "PrimitiveComponent Object Reference"))
  (`PrimitiveComponent.SetRenderCustomDepth` TouchedComponent true))

(event `self.Body.OnEndCursorOver`
  (params (TouchedComponent :type "PrimitiveComponent Object Reference"))
  (`PrimitiveComponent.SetRenderCustomDepth` TouchedComponent false))

(fn `AddCart`
  (params (Interactor :type "Actor Object Reference"))
  (returns (NewParam :type Boolean))
  (return false))

(fn `GetInteractableActions`
  (returns (Actions :type "Map of /Game/RoboSupport/Inventory/E_Tools Enum to String") (PuzzleRef :type "Actor Object Reference"))
  (return _ null))

(fn `GetInteractableType`
  (returns (NewParam :type "/Game/RoboSupport/Objects/E_InteractType Enum"))
  (return "NewEnumerator0"))

(fn `PuzzleInteract`
  (params (AnyTextIn :type String))
  (returns (AnyTextOut :type String))
  (return ""))

(fn `UserConstructionScript`)