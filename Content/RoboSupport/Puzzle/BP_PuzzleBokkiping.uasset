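; PC repair puzzle actor with clickable power supply, motherboard and power button, each given an attached particle effect at BeginPlay.
; Clicking a part passes its action list to a UI call; a helper function toggles an action widget at the cursor.
; Chosen actions update defect status and drain battery: Power On plays a sound once until Power Off resets it, Plug Mouse spawns a mouse and adds an inventory item.
; Several disconnected debug and battery snippets remain.
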(event `self.FixProblem`
  (params (Index :type Integer) (Status :type Boolean))
  (bind _problems (`self.Problems`))
  (`KismetArrayLibrary.Array_Set` _problems Index (make `/Game/RoboSupport/Puzzle/F_defects` (`.Name_10_7756C5F44B5E7448E29089A55EF04FFC` (break `/Game/RoboSupport/Puzzle/F_defects` (`|GetArrayItem` _problems Index))) Status)))

(event `self.SupplyUnit.OnClicked`
  (params (TouchedComponent :type "PrimitiveComponent Object Reference") (ButtonPressed :type "Key Structure"))
  ;[1 1 1] Вызов UI при нажатии на элемент и заполнение UI из массива ENUM
  (`self.CallUIOnClickElem` (`self.ActionSupplyUnit`)))

(event `self.ReceiveBeginPlay`
  (`parent.ReceiveBeginPlay`)
  (bind _returnvalue (`GameplayStatics.SpawnEmitterAttached` (`self.ET_SupplyUnit`) (`self.SupplyUnit`)))
  (set `self.SupplyUnitEffects` _returnvalue)
  (bind _returnvalue_2 (`GameplayStatics.SpawnEmitterAttached` (`self.ET_Motherboard`) (`self.MotherBoard`)))
  (set `self.MotherboardEffects` _returnvalue_2)
  (bind _returnvalue_3 (`GameplayStatics.SpawnEmitterAttached` (`self.ET_PowerButton`) (`self.PowerButton`)))
  (set `self.PowerButtonEffects` _returnvalue_3))

(event `self.PowerButton.OnClicked`
  (params (TouchedComponent :type "PrimitiveComponent Object Reference") (ButtonPressed :type "Key Structure"))
  ;[1 1 1] Вызов UI при нажатии на элемент и заполнение UI из массива ENUM
  (`self.CallUIOnClickElem` (`self.ActionPowerButton`)))

(event `self.MotherBoard.OnClicked`
  (params (TouchedComponent :type "PrimitiveComponent Object Reference") (ButtonPressed :type "Key Structure"))
  ;[1 1 1] Вызов UI при нажатии на элемент и заполнение UI из массива ENUM
  (`self.CallUIOnClickElem` (`self.ActionMoterboard`)))

(event `/Game/RoboSupport/Interface/BPI_Interact.PuzzleElemInteract`
  (params (Interactor :type "Actor Object Reference") (PbutoonAct :type "/Game/RoboSupport/Puzzle/E_ElemPButtonAct Enum" :default "NewEnumerator0"))
  (switch `/Game/RoboSupport/Puzzle/E_ElemPButtonAct` PbutoonAct
    (:`NewEnumerator0`
      (`self.FixProblem2` 0 true)
      (`self.Discharge Battery` 5.0)
      (`/Engine/EditorBlueprintResources/StandardMacros.DoOnce` false :!label _label
        (:`Completed`
          (`GameplayStatics.SpawnSound2D` "/Game/RoboSupport/Puzzle/Audio/PC_OnSound.PC_OnSound" 1.0 1.0 0.0 null))))
    (:`NewEnumerator1`
      (`self.FixProblem2` 0 true)
      (`self.Discharge Battery` 5.0)
      (goto _label :!via `Reset`))
    (:`NewEnumerator12`
      (`self.FixProblem2` 0)
      (`self.Discharge Battery` 5.0)
      (`|SpawnActorFromClass` "/Game/RoboSupport/Objects/BP_Mouse.BP_Mouse_C" (`self.GetTransform` (`self.SpawnPoint`)) "Undefined" "OverrideRootScale" null null)
      (bind _asbp_robot_support (cast `/Game/RoboSupport/Characters/BP_RobotSupport` (`GameplayStatics.GetPlayerPawn` 0)))
      (`/Game/RoboSupport/Inventory/AC_InventoriComponent.AddItem` (`/Game/RoboSupport/Characters/BP_RobotSupport.BPC_InventoriComponent` _asbp_robot_support) (`self.To Add`)))))

(fn `NewFunction_0_0`
  (params (Array :type "Array of /Game/RoboSupport/Puzzle/E_ElemPButtonAct Enum (by ref)"))
  (bind (_locationx _locationy) (`PlayerController.GetMousePosition` (`GameplayStatics.GetPlayerController` 0)))
  (bind _testui (`self.TestUI`)
    (:`then`
      (`Widget.RemoveFromParent` _testui)
      (set `self.TestUI` null))
    (:`else`
      (bind _returnvalue (`|CreateWidget` "/Game/RoboSupport/Puzzle/Widget/WBP_test.WBP_test_C" null self))
      (bind _output_get (set `self.TestUI` _returnvalue))
      (`UserWidget.AddToViewport` _output_get 0)
      (`/Game/RoboSupport/Puzzle/Widget/WBP_test.FillData` (`self.TestUI`) Array)
      ;[1 1 1] Вызов виджета рядом с курсором мышки
      (`UserWidget.SetPositionInViewport` (`self.TestUI`) (`KismetMathLibrary.MakeVector2D` _locationx _locationy) true))))

(fn `UserConstructionScript`
  (`parent.UserConstructionScript`))